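; Player-controlled Viking character with a spring-arm camera, able to interact with orbs and switch to the bird pawn when it is near.
; Tick drives camera-relative movement, scaled by a value that ramps with the running state.
; Capsule overlaps track the current orb or orb place for Interact and flag pushing of pushable objects and chess figures.
; It registers with the VikingGame instance, which handles pawn switching and reset, while a debug-style key changes the game mode.
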(event `self.ReceiveBeginPlay`
  ;[1 1 1] Initial Settings
  (set `self.bUseControllerRotationYaw` false)
  (set `SpringArmComponent.bUsePawnControlRotation` true (`self.SpringArm`))
  (set `CharacterMovementComponent.bOrientRotationToMovement` true (`self.CharacterMovement`))
  (`/Game/VikingProjectAssets/Blueprints/GameBPs/VikingGame.SetVikingPawn` (cast `/Game/VikingProjectAssets/Blueprints/GameBPs/VikingGame` (`GameplayStatics.GetGameInstance`) :!pure true) self)
  (set `self.currentMovementScaleValue` 0.5))

(event `self.ReceiveTick`
  (params (DeltaSeconds :type "Float (single-precision)"))
  ;[1 1 1] Movement
  (if (`self.Running`)
    (set `self.currentMovementScaleValue` (`KismetMathLibrary.FClamp` (+ (`self.currentMovementScaleValue`) (* (`GameplayStatics.GetWorldDeltaSeconds`) 0.5))))
    (else
      (set `self.currentMovementScaleValue` (`KismetMathLibrary.FClamp` (- (`self.currentMovementScaleValue`) (* (`GameplayStatics.GetWorldDeltaSeconds`) 0.83)) 0.17))))
  (`self.AddMovementInput` (`self.GetMoveDirection`)))

(event `InputAction|Interact`
  (params (Key :type "Key Structure"))
  ;[1 1 1] Consume Map orbs
  (:`Pressed`
    (if (!= (`self.CurrentOrb`) null)
      (`/Game/VikingProjectAssets/Blueprints/OrbBP.Consume Orb` (`self.CurrentOrb`))
      (else
        ;[1 1 1] Place orbs
        (if (!= (`self.CurrentOrbPlace`) null)
          (`/Game/VikingProjectAssets/Blueprints/OrbPlaceBP.Place Orb` (`self.CurrentOrbPlace`)))))))

(event `InputAxis|Turn` :overrideparent false
  (params (AxisValue :type "Float (single-precision)"))
  ;[1 1 1] Controller Input Parsing
  (`self.AddControllerYawInput` AxisValue))

(event `InputAction|Jump` :overrideparent false
  (params (Key :type "Key Structure"))
  ;[1 1 1] Controller Input Parsing
  (:`Pressed`
    (`self.Jump`))
  (:`Released`
    (`self.StopJumping`)))

(event `InputAxis|LookUp` :overrideparent false
  (params (AxisValue :type "Float (single-precision)"))
  ;[1 1 1] Controller Input Parsing
  (`self.AddControllerPitchInput` AxisValue))

(event `Key|M`
  (params (Key :type "Key Structure"))
  (:`Pressed`
    (`/Game/VikingProjectAssets/Blueprints/GameBPs/VikingGame.ResetPlayer` (cast `/Game/VikingProjectAssets/Blueprints/GameBPs/VikingGame` (`GameplayStatics.GetGameInstance`) :!pure true))))

(event `InputAction|Walk`
  (params (Key :type "Key Structure"))
  ;[1 1 1] Set Movement scale value
  (:`Pressed`
    (set `self.Running` true))
  (:`Released`
    (set `self.Running` false)))

(event `InputAction|SwitchView`
  (params (Key :type "Key Structure"))
  ;[1 1 1] Change To Bird
  (:`Released`
    (if (`self.BirdIsNear`)
      (`/Game/VikingProjectAssets/Blueprints/GameBPs/VikingGame.ChangePlayerPawn` (cast `/Game/VikingProjectAssets/Blueprints/GameBPs/VikingGame` (`GameplayStatics.GetGameInstance`) :!pure true) false))))

(event `self.CapsuleComponent.OnComponentBeginOverlap`
  (params (OverlappedComponent :type "PrimitiveComponent Object Reference") (OtherActor :type "Actor Object Reference") (OtherComp :type "PrimitiveComponent Object Reference") (OtherBodyIndex :type Integer) (bFromSweep :type Boolean) (SweepResult :type "HitResult Structure (by ref)"))
  ;[1 1 1] Overlap Events
  (bind _asorb_bp (cast `/Game/VikingProjectAssets/Blueprints/OrbBP` OtherActor)
    (:`then`
      (set `self.CurrentOrb` _asorb_bp))
    (:`CastFailed`
      (bind _asorb_place_bp (cast `/Game/VikingProjectAssets/Blueprints/OrbPlaceBP` OtherActor)
        (:`then`
          (set `self.CurrentOrbPlace` _asorb_place_bp))
        (:`CastFailed`
          (cast `/Game/VikingProjectAssets/Blueprints/PushableObject` OtherActor
            (:`then`
              _)
            (:`CastFailed`
              (cast `/Game/VikingProjectAssets/Blueprints/ChessFigure` OtherActor)))
          (set `self.PushingObject` true))))))

(event `self.CapsuleComponent.OnComponentEndOverlap`
  (params (OverlappedComponent :type "PrimitiveComponent Object Reference") (OtherActor :type "Actor Object Reference") (OtherComp :type "PrimitiveComponent Object Reference") (OtherBodyIndex :type Integer))
  ;[1 1 1] Overlap Events
  (cast `/Game/VikingProjectAssets/Blueprints/OrbBP` OtherActor
    (:`then`
      (set `self.CurrentOrb` null))
    (:`CastFailed`
      (cast `/Game/VikingProjectAssets/Blueprints/OrbPlaceBP` OtherActor
        (:`then`
          (set `self.CurrentOrbPlace` null))
        (:`CastFailed`
          (cast `/Game/VikingProjectAssets/Blueprints/PushableObject` OtherActor
            (:`then`
              _)
            (:`CastFailed`
              (cast `/Game/VikingProjectAssets/Blueprints/ChessFigure` OtherActor)))
          (set `self.PushingObject` false))))))

(event `self.Trigger.OnComponentBeginOverlap`
  (params (OverlappedComponent :type "PrimitiveComponent Object Reference") (OtherActor :type "Actor Object Reference") (OtherComp :type "PrimitiveComponent Object Reference") (OtherBodyIndex :type Integer) (bFromSweep :type Boolean) (SweepResult :type "HitResult Structure (by ref)"))
  ;[1 1 1] Check if bird is near
  (cast `/Game/VikingProjectAssets/Blueprints/GameBPs/BirdCharacter` OtherActor)
  (set `self.BirdIsNear` true))

(event `self.Trigger.OnComponentEndOverlap`
  (params (OverlappedComponent :type "PrimitiveComponent Object Reference") (OtherActor :type "Actor Object Reference") (OtherComp :type "PrimitiveComponent Object Reference") (OtherBodyIndex :type Integer))
  ;[1 1 1] Check if bird is near
  (cast `/Game/VikingProjectAssets/Blueprints/GameBPs/BirdCharacter` OtherActor)
  (set `self.BirdIsNear` false))

(event `Key|P`
  (params (Key :type "Key Structure"))
  (:`Pressed`
    (`/Game/VikingProjectAssets/Blueprints/Game/IcaroGameModeBP.ChangeModeEvt` (cast `/Game/VikingProjectAssets/Blueprints/Game/IcaroGameModeBP` (`GameplayStatics.GetGameMode`) :!pure true) "NewEnumerator2")))

(fn `GetMoveDirection`
  (returns (`Move Direction` :type "Vector Structure"))
  (bind _returnvalue (`self.GetControlRotation`))
  (return (* (`KismetMathLibrary.Normal` (+ (* (`KismetMathLibrary.GetForwardVector` _returnvalue) (`self.GetInputAxisValue`)) (* (`KismetMathLibrary.GetRightVector` _returnvalue) (`self.GetInputAxisValue`)))) (`self.currentMovementScaleValue`))))

(fn `UserConstructionScript`)