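; VikingGame is the central game-state Blueprint for possession switching, orb counts, respawn and saving.
; It stores Viking and Bird pawn references and has the player controller possess either one, or an enemy pawn via ChangeToEnemyCam.
; Placing an orb decrements the collected count, clamped at zero, while resetting possesses the Viking and teleports it to the current checkpoint.
; Saving writes the player transform and orb count to the ICARO_STATE slot.
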(fn `ChangePlayerPawn`
  (params (`I am Bird` :type Boolean :default false))
  (bind _returnvalue (`GameplayStatics.GetPlayerController` 0))
  (if `I am Bird`
    (`Controller.Possess` _returnvalue (`self.VikingPawn`))
    (else
      (`Controller.Possess` _returnvalue (`self.BirdPawn`)))))

(fn `ChangeToEnemyCam`
  (params (Pawn :type "/Game/VikingProjectAssets/Blueprints/NPC/IA-final/MiNPC_Escort_BP1 Object Reference"))
  (`Controller.Possess` (`GameplayStatics.GetPlayerController` 0) Pawn)
  (set `self.EnemyPawn` Pawn))

(fn `GetIsBird`
  (returns (isPlayerFlying :type Boolean))
  (return (== (`GameplayStatics.GetPlayerPawn` 0) (`self.BirdPawn`))))

(fn `PlaceOrb`
  (`/Engine/EditorBlueprintResources/StandardMacros.IncrementInt` (`self.PlacedOrbs`)
    (:`  `
      (`self.UpdateCollectedOrbs` 1 true))))

(fn `ResetPlayer`
  (`self.ChangePlayerPawn` true)
  (`SceneComponent.K2_SetWorldLocation` (`Actor.RootComponent` (`GameplayStatics.GetPlayerPawn` 0)) (`self.CurrentCheckPoint`) false true))

(fn `SaveOption`
  (bind _returnvalue (`GameplayStatics.CreateSaveGameObject` "/Game/VikingProjectAssets/Blueprints/Game/SaveIcaroBP.SaveIcaroBP_C"))
  (set `/Game/VikingProjectAssets/Blueprints/Game/SaveIcaroBP.Position` (`Actor.GetTransform` (`GameplayStatics.GetPlayerPawn` 0)) _returnvalue)
  (set `/Game/VikingProjectAssets/Blueprints/Game/SaveIcaroBP.Num_Orbs` (`self.CollectedOrbs`) _returnvalue)
  (`GameplayStatics.SaveGameToSlot` _returnvalue "ICARO_STATE"))

(fn `SetActualOrbs`
  (params (NumOrbsIHad :type Integer))
  (set `self.CollectedOrbs` NumOrbsIHad))

(fn `SetBirdPawn`
  (params (`Bird Pawn` :type "/Game/VikingProjectAssets/Blueprints/GameBPs/BirdCharacter Object Reference"))
  (set `self.BirdPawn` `Bird Pawn`))

(fn `SetVikingPawn`
  (params (`Viking Pawn` :type "/Game/VikingProjectAssets/Blueprints/GameBPs/VikingCharacter Object Reference"))
  (set `self.VikingPawn` `Viking Pawn`))

(fn `UpdateCollectedOrbs`
  (params (Quantity :type Integer :default 0) (`Substract Orbs` :type Boolean))
  (bind _returnvalue (- (`self.CollectedOrbs`) Quantity))
  (if `Substract Orbs`
    ;[1 1 1] Substract Orbs
    (if (<= _returnvalue 0)
      (set `self.CollectedOrbs` 0)
      (else
        (set `self.CollectedOrbs` _returnvalue)))
    (else
      ;[1 1 1] Add orbs
      (set `self.CollectedOrbs` (+ Quantity (`self.CollectedOrbs`))))))