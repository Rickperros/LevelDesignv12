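; BirdCharacter is the player's bird companion, flyable for a limited time in place of the Viking.
; While possessed, it constantly moves forward, with Jump setting climb or gravity, MoveRight steering and banking, and LookDown pitching the camera.
; The FlyTime timeline, restarted each flight, switches back to the Viking through the VikingGame instance when finished, as does SwitchView.
; Otherwise it interpolates above the player pawn, matching its rotation when overlapping the Viking.
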(event `self.ReceiveBeginPlay`
  ;[1 1 1] Initial Settings
  (set `self.bUseControllerRotationYaw` true)
  (set `CharacterMovementComponent.bOrientRotationToMovement` false (`self.CharacterMovement`))
  (set `self.InitialRotation` (`self.K2_GetActorRotation`))
  (`/Game/VikingProjectAssets/Blueprints/GameBPs/VikingGame.SetBirdPawn` (cast `/Game/VikingProjectAssets/Blueprints/GameBPs/VikingGame` (`GameplayStatics.GetGameInstance`) :!pure true) self))

(event `self.ReceiveTick`
  (params (DeltaSeconds :type "Float (single-precision)"))
  (bind _returnvalue (`GameplayStatics.GetPlayerPawn` 0))
  (bind _camera (`self.Camera`))
  (bind _relativerotation (`SceneComponent.RelativeRotation` _camera))
  (if (== (`self.GetController`) (`GameplayStatics.GetPlayerController` 0))
    (`|ExecutionSequence`
      (:`then_0`
        ;[1 1 1] Bird Movement
        (`self.AddMovementInput` (`self.GetMoveDirection`))
        (`self.K2_SetActorRotation` (`KismetMathLibrary.RInterpTo_Constant` (`self.K2_GetActorRotation`) (`KismetMathLibrary.MakeRotator` (+ (.roll (`self.InitialRotation`)) (* (`self.VeerRotation`) (`self.GetInputAxisValue`))) (.pitch (`self.K2_GetActorRotation`)) (.yaw (`self.K2_GetActorRotation`))) (`GameplayStatics.GetWorldDeltaSeconds`) (`self.VeerInterpSpeed`)))
        ;[1 1 1] Head Bow
        (`SceneComponent.K2_SetRelativeRotation` _camera (`KismetMathLibrary.RInterpTo_Constant` _relativerotation (`KismetMathLibrary.MakeRotator` (.roll _relativerotation) (* (`self.LookDown`) (`self.HeadMaxPitch`)) (.yaw _relativerotation)) (`GameplayStatics.GetWorldDeltaSeconds`) (`self.HeadBowInterpSpeed`)) false false))
      (:`then_1`
        ;[1 1 1] Change To Viking if Fly time has expired
        (if (`self.justStartFly`)
          (set `self.justStartFly` false)
          (bind (_direction _flytime) (`Timeline|FlyTime` :!via `PlayFromStart` :!label _label)
            (:`Update`
              (set `self.CurrentFlyTime` _flytime))
            (:`Finished`
              (`self.ChangeToViking`)))
          (else
            (goto _label)))))
    (else
      ;[1 1 1] Return to Player
      (`self.K2_SetActorLocation` (`KismetMathLibrary.VInterpTo` (`self.K2_GetActorLocation`) (+ (`self.K2_GetActorLocation` _returnvalue) (* (`self.GetActorUpVector` _returnvalue) 200.0)) (`GameplayStatics.GetWorldDeltaSeconds`) (`self.GetBackInterpolationSpeed`)))
      (if (`self.playerIsNear`)
        (`self.K2_SetActorRotation` (`self.K2_GetActorRotation` (`GameplayStatics.GetPlayerPawn` 0)))
        (else
          (`self.K2_SetActorRotation` (`KismetMathLibrary.MakeRotator` (.roll (`KismetMathLibrary.FindLookAtRotation` (`self.K2_GetActorLocation`) (`self.K2_GetActorLocation` (`GameplayStatics.GetPlayerPawn` 0)))) (.pitch (`self.K2_GetActorRotation`)) (.yaw (`KismetMathLibrary.FindLookAtRotation` (`self.K2_GetActorLocation`) (`self.K2_GetActorLocation` (`GameplayStatics.GetPlayerPawn` 0))))))))
      (set `self.justStartFly` true))))

(event `InputAction|SwitchView`
  (params (Key :type "Key Structure"))
  ;[1 1 1] Change to Viking
  (:`Released`
    (`/Game/VikingProjectAssets/Blueprints/GameBPs/VikingGame.ChangePlayerPawn` (cast `/Game/VikingProjectAssets/Blueprints/GameBPs/VikingGame` (`GameplayStatics.GetGameInstance`) :!pure true) true)))

(event `InputAxis|MoveRight`
  (params (AxisValue :type "Float (single-precision)"))
  ;[1 1 1] Input Parsing
  (`self.AddControllerYawInput` (* AxisValue (`self.VeerSmoother`))))

(event `InputAction|Jump`
  (params (Key :type "Key Structure"))
  ;[1 1 1] Input Parsing
  (:`Pressed`
    (set `self.FlyInput` (`self.FlyImpulse`)))
  (:`Released`
    (set `self.FlyInput` (`self.Gravity`))))

(event `ChangeToViking`
  ;[1 1 1] Change to Viking
  (`/Game/VikingProjectAssets/Blueprints/GameBPs/VikingGame.ChangePlayerPawn` (cast `/Game/VikingProjectAssets/Blueprints/GameBPs/VikingGame` (`GameplayStatics.GetGameInstance`) :!pure true) true))

(event `InputAction|LookDown`
  (params (Key :type "Key Structure"))
  ;[1 1 1] Input Parsing
  (:`Pressed`
    (set `self.LookDown` 1))
  (:`Released`
    (set `self.LookDown` 0)))

(event `self.ReceiveActorBeginOverlap`
  (params (OtherActor :type "Actor Object Reference"))
  ;[1 1 1] Check if player is near
  (cast `/Game/VikingProjectAssets/Blueprints/GameBPs/VikingCharacter` OtherActor)
  (set `self.playerIsNear` true))

(event `self.ReceiveActorEndOverlap`
  (params (OtherActor :type "Actor Object Reference"))
  ;[1 1 1] Check if player is near
  (cast `/Game/VikingProjectAssets/Blueprints/GameBPs/VikingCharacter` OtherActor)
  (set `self.playerIsNear` false))

(fn `GetMoveDirection`
  (returns (`Movement Direction` :type "Vector Structure"))
  (return (`KismetMathLibrary.Normal` (+ (* (`self.GetActorUpVector`) (`self.FlyInput`)) (`KismetMathLibrary.GetForwardVector` (`self.GetControlRotation`))))))

(fn `UserConstructionScript`)