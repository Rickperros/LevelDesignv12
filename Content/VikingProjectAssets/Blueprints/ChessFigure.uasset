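; ChessFigure is a physics chess piece actor that locks once it overlaps a TriggerVolume and then reacts to the VikingCharacter.
; Touching the volume marks its position as assigned and turns off physics simulation on the mesh.
; From then on, the character entering or leaving its Box toggles the ColorDefiner scalar on a dynamic material instance created in the construction script.
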(event `self.ReceiveActorBeginOverlap`
  (params (OtherActor :type "Actor Object Reference"))
  (cast `TriggerVolume` OtherActor)
  (set `self.PositionAsigned` true)
  (`PrimitiveComponent.SetSimulatePhysics` (`self.Mesh`) false))

(event `self.Box.OnComponentBeginOverlap`
  (params (OverlappedComponent :type "PrimitiveComponent Object Reference") (OtherActor :type "Actor Object Reference") (OtherComp :type "PrimitiveComponent Object Reference") (OtherBodyIndex :type Integer) (bFromSweep :type Boolean) (SweepResult :type "HitResult Structure (by ref)"))
  (cast `/Game/VikingProjectAssets/Blueprints/GameBPs/VikingCharacter` OtherActor)
  (if (`self.PositionAsigned`)
    (`MaterialInstanceDynamic.SetScalarParameterValue` (`self.Material`) "ColorDefiner" 0.0)))

(event `self.Box.OnComponentEndOverlap`
  (params (OverlappedComponent :type "PrimitiveComponent Object Reference") (OtherActor :type "Actor Object Reference") (OtherComp :type "PrimitiveComponent Object Reference") (OtherBodyIndex :type Integer))
  (cast `/Game/VikingProjectAssets/Blueprints/GameBPs/VikingCharacter` OtherActor)
  (if (`self.PositionAsigned`)
    (`MaterialInstanceDynamic.SetScalarParameterValue` (`self.Material`) "ColorDefiner" 1.0)))

(fn `UserConstructionScript`
  (bind _returnvalue (`KismetMaterialLibrary.CreateDynamicMaterialInstance` (`PrimitiveComponent.GetMaterial` (`self.Mesh`) 0)))
  (`PrimitiveComponent.SetMaterial` (`self.Mesh`) 0 _returnvalue)
  (set `self.Material` _returnvalue))