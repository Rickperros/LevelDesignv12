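; Door Blueprint that opens once the player has placed enough orbs, as counted by PlacedOrbs in the VikingGame game instance.
; Tick polls that count against RequiredPlacedOrbs, then creates and plays the Puerta1 level sequence once, caching the player in DoorSequence.
; When the sequence is no longer playing, Tick disables the mesh's collision and hides it rather than destroying the actor.
; A separate Destroy function removes the actor but is not called here.
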(event `self.ReceiveTick`
  (params (DeltaSeconds :type "Float (single-precision)"))
  (bind _staticmeshcomponent (`self.StaticMeshComponent`))
  (if (<= (`self.RequiredPlacedOrbs`) (`/Game/VikingProjectAssets/Blueprints/GameBPs/VikingGame.PlacedOrbs` (cast `/Game/VikingProjectAssets/Blueprints/GameBPs/VikingGame` (`GameplayStatics.GetGameInstance`) :!pure true)))
    (if (!= (`self.DoorSequence`) null)
      (if (not (`MovieSceneSequencePlayer.IsPlaying` (`self.DoorSequence`)))
        (`PrimitiveComponent.SetCollisionEnabled` _staticmeshcomponent "NoCollision")
        (`SceneComponent.SetVisibility` _staticmeshcomponent false false))
      (else
        (bind (_outactor _returnvalue) (`LevelSequencePlayer.CreateLevelSequencePlayer` "/Game/VikingProjectAssets/cinematicas/Puerta1.Puerta1"))
        (bind _output_get (set `self.DoorSequence` _returnvalue))
        (`MovieSceneSequencePlayer.Play` _output_get)))))

(fn `Destroy`
  (`self.K2_DestroyActor`))

(fn `UserConstructionScript`)