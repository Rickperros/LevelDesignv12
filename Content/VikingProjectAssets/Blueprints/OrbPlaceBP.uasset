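; OrbPlaceBP is an orb socket actor where the Viking player places collected orbs.
; A sphere overlap toggles a text prompt while a VikingCharacter is in range, with prompt and orb mesh hidden at start.
; PlaceOrb checks the game instance's collected orb count, calls its PlaceOrb, then plays a sound and reveals the orb.
; An unconnected leftover would play the Puerta1 level sequence.
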(event `self.ReceiveBeginPlay`
  (`SceneComponent.SetVisibility` (`self.TextRender`) false false)
  (`SceneComponent.SetVisibility` (`self.orb`) false false))

(event `self.Sphere.OnComponentBeginOverlap`
  (params (OverlappedComponent :type "PrimitiveComponent Object Reference") (OtherActor :type "Actor Object Reference") (OtherComp :type "PrimitiveComponent Object Reference") (OtherBodyIndex :type Integer) (bFromSweep :type Boolean) (SweepResult :type "HitResult Structure (by ref)"))
  (cast `/Game/VikingProjectAssets/Blueprints/GameBPs/VikingCharacter` OtherActor)
  (`SceneComponent.SetVisibility` (`self.TextRender`) true false))

(event `self.Sphere.OnComponentEndOverlap`
  (params (OverlappedComponent :type "PrimitiveComponent Object Reference") (OtherActor :type "Actor Object Reference") (OtherComp :type "PrimitiveComponent Object Reference") (OtherBodyIndex :type Integer))
  (cast `/Game/VikingProjectAssets/Blueprints/GameBPs/VikingCharacter` OtherActor)
  (`SceneComponent.SetVisibility` (`self.TextRender`) false false))

(fn `Place Orb`
  (bind _asviking_game (cast `/Game/VikingProjectAssets/Blueprints/GameBPs/VikingGame` (`GameplayStatics.GetGameInstance`) :!pure true))
  (if (> (`/Game/VikingProjectAssets/Blueprints/GameBPs/VikingGame.CollectedOrbs` _asviking_game) 0)
    (`/Game/VikingProjectAssets/Blueprints/GameBPs/VikingGame.PlaceOrb` _asviking_game)
    (`GameplayStatics.PlaySoundAtLocation` "/Game/VikingProjectAssets/Sounds/OrbPlace2.OrbPlace2" (`self.K2_GetActorLocation` self))
    (`SceneComponent.SetVisibility` (`self.orb`) true false)))

(fn `UserConstructionScript`)