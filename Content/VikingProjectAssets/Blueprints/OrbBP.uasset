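; OrbBP is a collectible orb that shows a text render while the VikingCharacter is near it.
; Trigger overlap events show and hide the text, which starts hidden on BeginPlay.
; ConsumeOrb, which is not called within this Blueprint, plays a sound at the orb's location, adds one to the collected orbs in the VikingGame game instance, then destroys the actor.
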(event `self.ReceiveBeginPlay`
  (`SceneComponent.SetVisibility` (`self.TextRender`) false false))

(event `self.Trigger.OnComponentBeginOverlap`
  (params (OverlappedComponent :type "PrimitiveComponent Object Reference") (OtherActor :type "Actor Object Reference") (OtherComp :type "PrimitiveComponent Object Reference") (OtherBodyIndex :type Integer) (bFromSweep :type Boolean) (SweepResult :type "HitResult Structure (by ref)"))
  (cast `/Game/VikingProjectAssets/Blueprints/GameBPs/VikingCharacter` OtherActor)
  (`SceneComponent.SetVisibility` (`self.TextRender`) true false))

(event `self.Trigger.OnComponentEndOverlap`
  (params (OverlappedComponent :type "PrimitiveComponent Object Reference") (OtherActor :type "Actor Object Reference") (OtherComp :type "PrimitiveComponent Object Reference") (OtherBodyIndex :type Integer))
  (cast `/Game/VikingProjectAssets/Blueprints/GameBPs/VikingCharacter` OtherActor)
  (`SceneComponent.SetVisibility` (`self.TextRender`) false false))

(fn `Consume Orb`
  (`GameplayStatics.SpawnSoundAtLocation` "/Game/VikingProjectAssets/Sounds/OrbSound__1_.OrbSound__1_" (`self.K2_GetActorLocation` self))
  (`/Game/VikingProjectAssets/Blueprints/GameBPs/VikingGame.UpdateCollectedOrbs` (cast `/Game/VikingProjectAssets/Blueprints/GameBPs/VikingGame` (`GameplayStatics.GetGameInstance`) :!pure true) 1 false)
  (`self.K2_DestroyActor`))

(fn `UserConstructionScript`)