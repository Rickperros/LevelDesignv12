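; A game instance Blueprint that holds an inventory struct with the key count and saved positions.
; AddKeys raises the key count, while ConsumeKeys deducts keys only when enough are held and returns whether it succeeded.
; SavePos writes the player pawn's transform and an escort NPC's transform into the same struct, taking the last MiNPC_Escort_BP1 actor found in the level.
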(fn `AddKeys`
  (params (NumKeys :type Integer))
  (setmembers `/Game/VikingProjectAssets/Blueprints/Game/SInventory` :`StructRef` (`self.Inventory`) :`NumKeys` (+ NumKeys (`.NumKeys_2_363995344A89B99F24BFD99BBF8E8A0C` (break `/Game/VikingProjectAssets/Blueprints/Game/SInventory` (`self.Inventory`)))))
  (return))

(fn `ConsumeKeys`
  (params (NumKeys :type Integer))
  (returns (Success :type Boolean))
  (if (<= NumKeys (`.NumKeys_2_363995344A89B99F24BFD99BBF8E8A0C` (break `/Game/VikingProjectAssets/Blueprints/Game/SInventory` (`self.Inventory`))))
    (setmembers `/Game/VikingProjectAssets/Blueprints/Game/SInventory` :`StructRef` (`self.Inventory`) :`NumKeys` (- (`.NumKeys_2_363995344A89B99F24BFD99BBF8E8A0C` (break `/Game/VikingProjectAssets/Blueprints/Game/SInventory` (`self.Inventory`))) NumKeys))
    (return true)
    (else
      (return false))))

(fn `SavePos`
  (bind _outactors (`GameplayStatics.GetAllActorsOfClass` "/Game/VikingProjectAssets/Blueprints/NPC/IA-final/MiNPC_Escort_BP1.MiNPC_Escort_BP1_C"))
  (for _array_element _outactors
    _)
  (setmembers `/Game/VikingProjectAssets/Blueprints/Game/SInventory` :`StructRef` (`self.Inventory`) :`SavedPosPlayer` (`Actor.GetTransform` (`GameplayStatics.GetPlayerPawn` 0)) :`SavedPosNPC` (`Actor.GetTransform` _array_element))
  (return))