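; Final door Blueprint that opens once enough orbs have been placed in the game.
; Each Tick compares RequiredPlacedOrbs with the PlacedOrbs count on the VikingGame game instance.
; When the count is met, it deactivates and hides the Door component, then creates and plays a Puerta1 level sequence player.
; No one-shot guard exists, so this repeats every frame while the condition holds.
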(event `self.ReceiveTick`
  (params (DeltaSeconds :type "Float (single-precision)"))
  (bind _door (`self.Door`))
  (if (<= (`self.RequiredPlacedOrbs`) (`/Game/VikingProjectAssets/Blueprints/GameBPs/VikingGame.PlacedOrbs` (cast `/Game/VikingProjectAssets/Blueprints/GameBPs/VikingGame` (`GameplayStatics.GetGameInstance`) :!pure true)))
    (`ActorComponent.SetActive` _door false false)
    (`SceneComponent.SetVisibility` _door false false)
    (bind _outactor (`LevelSequencePlayer.CreateLevelSequencePlayer` "/Game/VikingProjectAssets/cinematicas/Puerta1.Puerta1"))
    (`MovieSceneSequencePlayer.Play` (`LevelSequenceActor.SequencePlayer` _outactor))))

(fn `UserConstructionScript`)