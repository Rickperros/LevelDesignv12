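; NPC1 is an NPC Blueprint that writes the Target key of its AI Blackboard every Tick.
; Its Branch is meant to switch Target between null when far and the player pawn when near, with debug prints for each case.
; The 1000-unit distance check is not wired to the Branch, whose condition is fixed true, so Target is always cleared.
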(event `self.ReceiveTick`
  (params (DeltaSeconds :type "Float (single-precision)"))
  (bind _returnvalue (`AIBlueprintHelperLibrary.GetBlackboard` null))
  (if true
    (`KismetSystemLibrary.PrintText` "MuyLejos")
    (`BlackboardComponent.SetValueAsObject` _returnvalue "Target" (`self.Null`))
    (else
      (`KismetSystemLibrary.PrintString` "Cerca")
      (`BlackboardComponent.SetValueAsObject` _returnvalue "Target" (`GameplayStatics.GetPlayerPawn` 0)))))

(fn `UserConstructionScript`)